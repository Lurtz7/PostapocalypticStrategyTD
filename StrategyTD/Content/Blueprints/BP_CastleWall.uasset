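; BP_CastleWall is a destructible castle wall segment that takes damage and spreads part of it to nearby walls.
; WALLGOTHIT reduces its Health, updates its HP text, then searches all BP_CastleWall actors for others within a fixed radius, printing their distances.
; Those neighbors are gathered in a temporary array, lose half as much Health and update their text.
; Any wall reaching zero Health is destroyed.
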(event Custom|WALL%20GOT%20HIT
  (bind _surroundingwalls (Variables|Default|GetSurroundingWalls))
  (Variables|Default|SetHealth (- (Variables|Default|GetHealth) 250))
  (Rendering|Components|TextRender|SetText (Variables|Default|GetHP_TEXT) (Utilities|Text|ToText(Integer) (Variables|Default|GetHealth)))
  (bind _outactors (Actor|GetAllActorsOfClass "BP_CastleWall_C"))
  (for _array_element _outactors
    (if (Utilities|Enum|NotEqual(Enum) (Utilities|GetDisplayName _array_element) (Utilities|GetDisplayName self))
      (if (<= (Transformation|GetDistanceTo self _array_element) 7e+02)
        (Development|PrintString (Utilities|String|ToString(Float) (Transformation|GetDistanceTo self _array_element)))
        (Utilities|Array|Add (Variables|Default|GetSurroundingWalls) _array_element))))
  (for _array_element_2 _surroundingwalls
    (Variables|BP_CastleWall_C|SetHealth _array_element_2 (- (Variables|BP_CastleWall_C|GetHealth _array_element_2) 125))
    (Rendering|Components|TextRender|SetText (Variables|BP_CastleWall_C|GetHP_TEXT _array_element_2) (Utilities|Text|ToText(Integer) (Variables|BP_CastleWall_C|GetHealth _array_element_2)))
    (if (<= (Variables|BP_CastleWall_C|GetHealth _array_element_2) 0)
      (Actor|DestroyActor _array_element_2)))
  (Utilities|Array|Clear _surroundingwalls)
  (if (<= (Variables|Default|GetHealth) 0)
    (Actor|DestroyActor)))

(fn ConstructionScript)