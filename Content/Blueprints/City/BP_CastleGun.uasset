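; Castle gun turret actor that automatically shoots at nearby actors tagged "Enemy".
; Tick, gated by a short Delay, gathers tagged actors and appends those within range to a close list, cleared after firing.
; The turret top interpolates toward an indexed entry in the full enemy list, while a visibility trace targets a random-indexed close enemy.
; Any trace hit spawns muzzle effect, sound and TurretBullet at the muzzle socket; IdleScan is empty.
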(event EventTick
  (params (DeltaSeconds :type Float%20%28single-precision%29))
  (bind _self self)
  (bind _enemyclose (Variables|Default|GetENEMYCLOSE))
  (bind _enemyclose_2 (Variables|Default|GetENEMYCLOSE))
  (bind _castlegun_turret_top_001 (Variables|Default|GetCastleGun_Turret_Top_001 _self))
  (bind _returnvalue (Transformation|GetSocketLocation _castlegun_turret_top_001 "Mynning"))
  (bind _returnvalue_2 (Transformation|GetSocketTransform _castlegun_turret_top_001 "Mynning" "RTS_World"))
  (bind (_location _rotation) (Math|Transform|BreakTransform _returnvalue_2))
  (Utilities|FlowControl|Delay 0.1)
  (bind _outactors (Actor|GetAllActorswithTag "Enemy"))
  (bind _output_get (Variables|Default|SetENEMY _outactors))
  (for _array_element _output_get
    (if (< (Transformation|GetDistanceTo _array_element _self) 7e+03)
      (Utilities|Array|Add _enemyclose _array_element)))
  (if (== (Utilities|Array|Length _enemyclose_2) 0)
    (Utilities|Array|Clear (Variables|Default|GetENEMYCLOSE))
    (else
      (CallFunction|RotateTowardsTarget)
      (bind (_outhit _returnvalue_3) (Collision|LineTraceByChannel _returnvalue (Transformation|GetActorLocation (Utilities|Array|Get(acopy) _enemyclose_2 (Math|Random|RandomInteger (Variables|Default|GetTargetIndex)))) "TraceTypeQuery1" false 0 "None" true "(R=1.000000,G=0.000000,B=0.000000,A=1.000000)" "(R=0.000000,G=1.000000,B=0.000000,A=1.000000)" 5e+01))
      (if _returnvalue_3
        (Effects|SpawnEmitteratLocation "/Game/StarterContent/Particles/P_EXPLTurret.P_EXPLTurret" _returnvalue "0, 0, 0" "0.500000,0.500000,0.500000")
        (Audio|SpawnSoundatLocation "/Engine/VREditor/Sounds/UI/Flashlight_Switch.Flashlight_Switch" _returnvalue "0, 0, 0" 1.0 1.0 0.0 0 0)
        (Game|SpawnActorfromClass "/Game/Blueprints/Tank/TurretBullet.TurretBullet_C" (Math|Transform|MakeTransform (+ _location "0, 0, 0") _rotation "0.400000,0.400000,0.400000") "AlwaysSpawn" 0 self)
        (Utilities|Array|Clear _enemyclose)))))

(fn ConstructionScript)

(fn RotateTowardsTarget
  (bind _castlegun_turret_top_001 (Variables|Default|GetCastleGun_Turret_Top_001))
  (Transformation|SetWorldRotation (Variables|Default|GetCastleGun_Turret_Top_001) (Math|Interpolation|RInterpTo (Transformation|GetWorldRotation _castlegun_turret_top_001) (Math|Rotator|FindLookatRotation (Transformation|GetWorldLocation _castlegun_turret_top_001) (Transformation|GetActorLocation (Utilities|Array|Get(acopy) (Variables|Default|GetENEMY) (Variables|Default|GetTargetIndex)))) (Utilities|Time|GetWorldDeltaSeconds) 1.5e+02) false false))

(fn IdleScan)