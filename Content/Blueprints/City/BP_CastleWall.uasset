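; BP_CastleWall is a destructible city castle wall segment with health shown on a widget progress bar and text.
; WALLGOTHIT deals fixed damage to the hit wall and half as much to other walls found nearby through an all-actors distance search.
; Each affected wall's display is refreshed, and depleted walls are destroyed.
; The hit wall sets its own WallDown flag when it or any damaged neighbour falls.
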(event Custom|WALL%20GOT%20HIT
  (bind _surroundingwalls (Variables|Default|GetSurroundingWalls))
  (bind _output_get (Variables|Default|SetHealth (- (Variables|Default|GetHealth) 250)))
  (bind _ashp_wall (Utilities|Casting|CastToHP_WALL (UserInterface|GetUserWidgetObject (Variables|Default|GetWidget))))
  (Progress|SetPercent (Variables|/Game/Blueprints/UserInterface/HP_WALL.HP_WALL_C|GetProgressBar_79 _ashp_wall) (/ (Math|Conversions|ToFloat(Integer) _output_get) 1.5e+03))
  (Rendering|Components|TextRender|SetText (Variables|Default|GetHP_TEXT) (Utilities|Text|ToText(Integer) (Variables|Default|GetHealth)))
  (bind _outactors (Actor|GetAllActorsOfClass "BP_CastleWall_C"))
  (for _array_element _outactors
    (if (Utilities|Enum|NotEqual(Enum) (Utilities|GetDisplayName _array_element) (Utilities|GetDisplayName self))
      (if (<= (Transformation|GetDistanceTo self _array_element) 7e+02)
        (Utilities|Array|Add (Variables|Default|GetSurroundingWalls) _array_element))))
  (for _array_element_2 _surroundingwalls
    (bind _output_get_2 (Variables|BP_CastleWall_C|SetHealth _array_element_2 (- (Variables|BP_CastleWall_C|GetHealth _array_element_2) 125)))
    (bind _ashp_wall_2 (Utilities|Casting|CastToHP_WALL (UserInterface|GetUserWidgetObject (Variables|BP_CastleWall_C|GetWidget _array_element_2))))
    (Progress|SetPercent (Variables|/Game/Blueprints/UserInterface/HP_WALL.HP_WALL_C|GetProgressBar_79 _ashp_wall_2) (/ (Math|Conversions|ToFloat(Integer) _output_get_2) 1.5e+03))
    (Rendering|Components|TextRender|SetText (Variables|BP_CastleWall_C|GetHP_TEXT _array_element_2) (Utilities|Text|ToText(Integer) (Variables|BP_CastleWall_C|GetHealth _array_element_2)))
    (if (<= (Variables|BP_CastleWall_C|GetHealth _array_element_2) 0)
      (Variables|Default|SetWallDown true)
      (Actor|DestroyActor _array_element_2)))
  (Utilities|Array|Clear _surroundingwalls)
  (if (<= (Variables|Default|GetHealth) 0)
    (Variables|Default|SetWallDown true)
    (Actor|DestroyActor)))

(fn ConstructionScript)