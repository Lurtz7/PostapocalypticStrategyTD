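; AI tank Blueprint that aims at an Origin point and fires shells, flagging breaches in the castle wall.
; Tick eases the turret mesh toward Origin while the tank is moving; a separate function does the same for the whole actor.
; TankShoot traces from the Nozzle socket and, on a hit, spawns a bullet toward it with explosion effects.
; It then sets BreachInWall if the BP_CastleWall count differs from twenty.
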(event EventTick
  (params (DeltaSeconds :type Float%20%28single-precision%29))
  (CallFunction|SetTurretRotation))

(fn ConstructionScript)

(fn TankShoot
  (bind _tankmodelsep_drawcall_1311 (Variables|Default|GettankModelSep_DrawCall_1311))
  (bind _tankmodelsep_drawcall_1311_2 (Variables|Default|GettankModelSep_DrawCall_1311))
  (bind _returnvalue (Transformation|GetSocketTransform _tankmodelsep_drawcall_1311_2 "Nozzle" "RTS_World"))
  (bind (_location _rotation) (Math|Transform|BreakTransform _returnvalue))
  (bind (_x _y) (Math|Rotator|GetAxes _rotation))
  (bind (_outhit _returnvalue_2) (Collision|LineTraceByChannel (Transformation|GetSocketLocation _tankmodelsep_drawcall_1311 "Nozzle") (+ (Transformation|GetSocketLocation _tankmodelsep_drawcall_1311 "None") (* (Math|Vector|GetForwardVector (Math|Rotator|MakeRotationfromAxes _x _y (.Z (Math|Rotator|BreakRotIntoAxes (Transformation|GetWorldRotation (Variables|Collision|GetCapsuleComponent)))))) 4e+04)) "TraceTypeQuery1" false 0 "None" true "(R=1.000000,G=0.000000,B=0.000000,A=1.000000)" "(R=0.000000,G=1.000000,B=0.000000,A=1.000000)" 5e+01))
  (if _returnvalue_2
    (Game|SpawnActorfromClass "/Game/Blueprints/Tank/Bullet.Bullet_C" (Math|Transform|MakeTransform (+ _location "0, 0, 0") (Math|Rotator|FindLookatRotation _location (.Location (Collision|BreakHitResult _outhit)))) "AlwaysSpawn" 0 self)
    (Components|Activation|Activate (Variables|Default|GetExplosion) false)
    (Components|Activation|Activate (Variables|Default|GetExplosionAudio) false)
    (bind _outactors (Actor|GetAllActorsOfClass "/Game/Blueprints/BP_CastleWall.BP_CastleWall_C"))
    (if (not (== (Utilities|Array|Length _outactors) 20))
      (bind _output_get (Variables|Default|SetBreachInWall true))
      (Development|PrintString (Utilities|String|ToString(Integer) (Utilities|Array|Length _outactors)) true true "(R=1.000000,G=0.000000,B=0.117299,A=1.000000)" 5.0))))

(fn SetBaseRotation
  (Transformation|SetActorRotation (Math|Interpolation|RInterpTo (Transformation|GetActorRotation) (Math|Rotator|FindLookatRotation (Transformation|GetActorLocation self) (Variables|Default|GetOrigin)) (Utilities|Time|GetWorldDeltaSeconds) 1.0)))

(fn SetTurretRotation
  (bind _tankmodelsep_drawcall_1311 (Variables|Default|GettankModelSep_DrawCall_1311))
  (if (not (Math|Vector|Equal(Vector) (Transformation|GetComponentVelocity (Variables|Collision|GetCapsuleComponent)) "0, 0, 0" 1e+02))
    (Transformation|SetWorldRotation _tankmodelsep_drawcall_1311 (Math|Interpolation|RInterpTo (Transformation|GetWorldRotation _tankmodelsep_drawcall_1311) (Math|Rotator|FindLookatRotation (Transformation|GetWorldLocation _tankmodelsep_drawcall_1311) (Variables|Default|GetOrigin)) (Utilities|Time|GetWorldDeltaSeconds) 1.0) false false)))