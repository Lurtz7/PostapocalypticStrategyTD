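; Behavior tree task, in the Tank folder, that picks a randomized destination near a north castle wall and writes it to the blackboard.
; It gathers all BP_CastleWall actors and appends those with "North" in their display name to FinalTarget, which it never clears.
; Random picks from the first five entries supply the location, which is shifted along +Y and jittered in X/Y.
; A separately rolled wall name is printed for debugging.
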(event EventReceiveExecuteAI
  (params (OwnerController :type AI%20Controller%20Object%20Reference) (ControlledPawn :type Pawn%20Object%20Reference))
  (bind _returnvalue (Math|Random|RandomIntegerinRange 0 4))
  (bind _returnvalue_2 (Math|Random|RandomFloatinRange -5e+02 5e+02))
  (bind _finaltarget (Variables|Default|GetFinalTarget))
  (bind _output (Utilities|Array|Get(acopy) _finaltarget _returnvalue))
  (bind _returnvalue_3 (Transformation|GetActorLocation _output))
  (bind (_x _y _z) (Math|Vector|BreakVector _returnvalue_3))
  (bind _outactors (Actor|GetAllActorsOfClass "/Game/Blueprints/BP_CastleWall.BP_CastleWall_C"))
  (bind _output_get (Variables|Default|SetTargetArray _outactors))
  (for _array_element _output_get
    (if (Utilities|String|Contains (Utilities|GetDisplayName _array_element) "North")
      (Utilities|Array|Add (Variables|Default|GetFinalTarget) _array_element)))
  (Development|PrintString (Utilities|GetDisplayName _output))
  (AI|BehaviorTree|SetBlackboardValueasVector (Variables|Default|GetVect) (+ (Math|Vector|MakeVector _x (+ _y 4e+03) _z) (Math|Vector|MakeVector _returnvalue_2 _returnvalue_2 0.0)))
  (AI|BehaviorTree|FinishExecute true))