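; Target is an actor that marks a stopping point for AI units.
; When an actor begins overlapping its Box component, it compares the exact class against AngryAI and BP_TankAI and clears IsMoving on a match.
; An AngryAI also gets a LookAtStructure call, while a BP_TankAI only stops.
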(event OnComponentBeginOverlap(Box)
  (params (OverlappedComponent :type Primitive%20Component%20Object%20Reference) (OtherActor :type Actor%20Object%20Reference) (OtherComp :type Primitive%20Component%20Object%20Reference) (OtherBodyIndex :type Integer) (bFromSweep :type Boolean) (SweepResult :type Hit%20Result%20Structure%20%28by%20ref%29))
  (if (== (Utilities|GetClass OtherActor) "/Game/Blueprints/AngryAI.AngryAI_C")
    (bind _asangry_ai (Utilities|Casting|CastToAngryAI OtherActor))
    (Variables|/Game/Blueprints/AngryAI.AngryAI_C|SetisMoving _asangry_ai false)
    (Default|LookatStructure _asangry_ai)
    (elif (== (Utilities|GetClass OtherActor) "/Game/Blueprints/BP_TankAI.BP_TankAI_C")
      (bind _asbp_tank_ai (Utilities|Casting|CastToBP_TankAI OtherActor))
      (Variables|/Game/Blueprints/BP_TankAI.BP_TankAI_C|SetisMoving _asbp_tank_ai false))))

(fn ConstructionScript)