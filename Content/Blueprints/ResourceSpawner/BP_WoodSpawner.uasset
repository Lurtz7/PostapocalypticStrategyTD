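; BP_WoodSpawner is a spawner actor that scatters wood resource actors inside its Box component's volume.
; On BeginPlay it loops to spawn a fixed batch of BP_WOOD at random points within the box bounds, with no rotation.
; Tick is empty, and disconnected leftover nodes hold an unused delayed, tag-count-capped random spawner for wood and stone, plus a stray food spawn.
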(event EventTick
  (params (DeltaSeconds :type Float%20%28single-precision%29)))

(event EventBeginPlay
  (bind _box (Variables|Default|GetBox))
  (for _index (range 0 25)
    (Game|SpawnActorfromClass "/Game/Blueprints/ResourceSpawner/BP_WOOD.BP_WOOD_C" (Math|Transform|MakeTransform (Math|Random|RandomPointinBoundingBox (Transformation|GetWorldLocation _box) (Variables|/Script/Engine.BoxComponent|GetBoxExtent _box)) "0, 0, 0" "1.000000,1.000000,1.000000") "Undefined" 0 0)))

(fn ConstructionScript)