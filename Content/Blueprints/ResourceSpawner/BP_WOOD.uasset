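; BP_WOOD is a harvestable wood resource actor that holds a random amount of wood.
; On BeginPlay it traces down at its XY position, snaps to the hit point and randomizes its yaw and per-axis scale.
; It destroys itself if the traced actor is tagged Water or Resources.
; RemoveWood decrements the count by one and destroys the actor once none remains.
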(event EventBeginPlay
  (bind _returnvalue (Transformation|GetActorTransform))
  (bind _returnvalue_2 (Math|Random|RandomIntegerinRange 5 15))
  (bind _location (Math|Transform|BreakTransform _returnvalue))
  (bind _location_2 (Math|Transform|BreakTransform _returnvalue))
  (bind _returnvalue_3 (Math|Conversions|ToFloat(Integer) _returnvalue_2))
  (bind (_x _y) (Math|Vector|BreakVector _location_2))
  (bind _returnvalue_4 (/ _returnvalue_3 4.0))
  (bind (_x_2 _y_2) (Math|Vector|BreakVector _location))
  (Variables|Default|SetWood%20Resources _returnvalue_2)
  (bind _outhit (Collision|LineTraceByChannel (Math|Vector|MakeVector _x _y 4e+02) (Math|Vector|MakeVector _x _y -1e+03) "TraceTypeQuery1" false 0 "None" true "(R=1.000000,G=0.000000,B=0.000000,A=1.000000)" "(R=0.000000,G=1.000000,B=0.000000,A=1.000000)" 15.0))
  (Transformation|SetActorTransform (Math|Transform|MakeTransform (.ImpactPoint (Collision|BreakHitResult _outhit)) (Math|Rotator|MakeRotator 0.0 0.0 (Math|Random|RandomFloatinRange 0.0 3.6e+02)) (.Scale (Math|Transform|BreakTransform (Math|Transform|MakeTransform (Math|Vector|MakeVector _x_2 _y_2 1.4e+02) "0, 0, 0" (Math|Vector|MakeVector _returnvalue_4 _returnvalue_4 _returnvalue_4))))))
  (if (or (Actor|ActorHasTag (.HitActor (Collision|BreakHitResult _outhit)) "Water") (Actor|ActorHasTag (.HitActor (Collision|BreakHitResult _outhit)) "Resources"))
    (Actor|DestroyActor)))

(fn ConstructionScript)

(fn RemoveWood
  (Variables|Default|SetWood%20Resources (- (Variables|Default|GetWood%20Resources) 1))
  (if (<= (Variables|Default|GetWood%20Resources) 0)
    (Actor|DestroyActor)))