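; Resource spawner actor that scatters wood and stone pickups at random points within its Box component's flattened, 100x-scaled extent.
; BeginPlay spawns an initial random batch and prints a sample point for debugging.
; Tick uses a Delay to attempt periodic spawns while actors tagged "Resources" number below a cap, with one random outcome spawning nothing.
; Food spawn nodes exist but are disconnected.
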(event EventTick
  (params (DeltaSeconds :type Float%20%28single-precision%29))
  (bind _box (Variables|Default|GetBox))
  (bind _returnvalue (Transformation|GetWorldLocation _box))
  (bind _boxextent (Variables|/Script/Engine.BoxComponent|GetBoxExtent _box))
  (bind (_x _y) (Math|Vector|BreakVector _boxextent))
  (bind _returnvalue_2 (Math|Vector|MakeVector _x _y 0.0))
  (bind _returnvalue_3 (* _returnvalue_2 1e+02))
  (bind _returnvalue_4 (Math|Random|RandomPointinBoundingBox _returnvalue _returnvalue_3))
  (bind _returnvalue_5 (Math|Transform|MakeTransform _returnvalue_4 "0, 0, 0" "1.000000,1.000000,1.000000"))
  (bind _outactors (Actor|GetAllActorswithTag "Resources"))
  (if (not (>= (Utilities|Array|Length _outactors) 50))
    (Utilities|FlowControl|Delay 5.0)
    (Development|PrintString (Utilities|String|ToString(Vector) _boxextent))
    (switch int (Math|Random|RandomIntegerinRange 0 2)
      (:0
        (Game|SpawnActorfromClass "/Game/Blueprints/ResourceSpawner/BP_WOOD.BP_WOOD_C" _returnvalue_5 "Undefined" 0 0))
      (:1
        (Game|SpawnActorfromClass "/Game/Blueprints/ResourceSpawner/BP_STONE1.BP_STONE1_C" _returnvalue_5 "Undefined" 0 0)))))

(event EventBeginPlay
  (bind _box (Variables|Default|GetBox))
  (bind _returnvalue (Transformation|GetWorldLocation _box))
  (bind _boxextent (Variables|/Script/Engine.BoxComponent|GetBoxExtent _box))
  (bind (_x _y) (Math|Vector|BreakVector _boxextent))
  (bind _returnvalue_2 (Math|Vector|MakeVector _x _y 0.0))
  (bind _returnvalue_3 (* _returnvalue_2 1e+02))
  (bind _returnvalue_4 (Math|Random|RandomPointinBoundingBox _returnvalue _returnvalue_3))
  (bind _returnvalue_5 (Math|Transform|MakeTransform _returnvalue_4 "0, 0, 0" "1.000000,1.000000,1.000000"))
  (for _index (range 0 11)
    (switch int (Math|Random|RandomIntegerinRange 0 1)
      (:0
        (Game|SpawnActorfromClass "/Game/Blueprints/ResourceSpawner/BP_WOOD.BP_WOOD_C" _returnvalue_5 "Undefined" 0 0))
      (:1
        (Game|SpawnActorfromClass "/Game/Blueprints/ResourceSpawner/BP_STONE1.BP_STONE1_C" _returnvalue_5 "Undefined" 0 0))))
  (Development|PrintString (Utilities|String|ToString(Vector) _returnvalue_4)))

(fn ConstructionScript)