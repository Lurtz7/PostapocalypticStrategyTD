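; BP_FOOD1 is a depletable food resource actor that varies its stock and footprint per instance.
; On BeginPlay it rolls a random food count, snaps to a fixed height with zero rotation, and randomizes X and Y scale independently of that count.
; The random ranges have Min and Max reversed.
; RemoveFoodResource takes one unit per call and destroys the actor when none remain.
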(event EventBeginPlay
  (bind _returnvalue (Transformation|GetActorTransform))
  (bind _returnvalue_2 (Math|Random|RandomIntegerinRange 15 5))
  (bind _location (Math|Transform|BreakTransform _returnvalue))
  (bind _returnvalue_3 (Math|Conversions|ToFloat(Integer) _returnvalue_2))
  (bind _returnvalue_4 (/ _returnvalue_3 5.0))
  (bind (_x _y) (Math|Vector|BreakVector _location))
  (Variables|Default|SetFoodResources _returnvalue_2)
  (Transformation|SetActorTransform (Math|Transform|MakeTransform (Math|Vector|MakeVector _x _y 1.4e+02) "0, 0, 0" (Math|Vector|MakeVector _returnvalue_4 _returnvalue_4 1.0))))

(fn ConstructionScript)

(fn RemoveFoodResource
  (Variables|Default|SetFoodResources (- (Variables|Default|GetFoodResources) 1))
  (if (<= (Variables|Default|GetFoodResources) 0)
    (Actor|DestroyActor)))