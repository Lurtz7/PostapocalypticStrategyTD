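; Allied unit character for a strategy game that automatically gathers nearby food, wood and stone.
; Tick swaps the ActivatedSymbol material to reflect selection and starts three parallel Delay nodes that throttle the resource checks to about every three seconds.
; Each check scans all actors of its resource type for those within range, calls the removal function on the resource, credits StrategyGameModeBase, and clears its array inside the loop.
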(event EventTick
  (params (DeltaSeconds :type Float%20%28single-precision%29))
  (bind _activatedsymbol (Variables|Default|GetActivatedSymbol))
  (if (Variables|Default|GetisSelectionActivated)
    (Rendering|Material|SetMaterial _activatedsymbol 0 "/Engine/MapTemplates/Materials/BasicAsset01.BasicAsset01")
    (else
      (Rendering|Material|SetMaterial _activatedsymbol 0 "/Engine/VREditor/UI/ArrowMaterial.ArrowMaterial")))
  (if true
    (Utilities|FlowControl|Sequence
      (:then_0
        (Utilities|FlowControl|Delay 3.0)
        (CallFunction|CheckFood))
      (:then_1
        (Utilities|FlowControl|Delay 3.0)
        (CallFunction|CheckWood))
      (:then_2
        (Utilities|FlowControl|Delay 3.0)
        (CallFunction|CheckStone)))))

(fn ConstructionScript)

(fn CheckFood
  (bind _food_resource (Variables|Default|GetFood_Resource))
  (bind _outactors (Actor|GetAllActorsOfClass "/Game/Blueprints/ResourceSpawner/BP_FOOD1.BP_FOOD1_C"))
  (for _array_element _outactors
    (if (<= (Transformation|GetDistanceTo _array_element) 7e+02)
      (Utilities|Array|Add (Variables|Default|GetFood_Resource) _array_element)))
  (for (_ _array_index) _food_resource
    (if (<= (Transformation|GetDistanceTo (Utilities|Array|Get(acopy) _food_resource _array_index)) 7e+02)
      (Default|RemoveFoodResource (Utilities|Array|Get(acopy) _food_resource _array_index))
      (bind _returnvalue (Actor|GetActorOfClass "/Game/MainGameModeBP/StrategyGameModeBase.StrategyGameModeBase_C"))
      (Default|AddFoodtoMain _returnvalue)
      (Utilities|Array|Clear (Variables|Default|GetFood_Resource)))))

(fn CheckWood
  (bind _wood_resource (Variables|Default|GetWood_Resource))
  (bind _outactors (Actor|GetAllActorsOfClass "/Game/Blueprints/ResourceSpawner/BP_WOOD.BP_WOOD_C"))
  (for _array_element _outactors
    (if (<= (Transformation|GetDistanceTo _array_element) 7e+02)
      (Utilities|Array|Add (Variables|Default|GetWood_Resource) _array_element)))
  (for (_ _array_index) _wood_resource
    (if (<= (Transformation|GetDistanceTo (Utilities|Array|Get(acopy) _wood_resource _array_index)) 7e+02)
      (Default|RemoveWood (Utilities|Array|Get(acopy) _wood_resource _array_index))
      (bind _returnvalue (Actor|GetActorOfClass "/Game/MainGameModeBP/StrategyGameModeBase.StrategyGameModeBase_C"))
      (Default|AddWoodtoMain _returnvalue)
      (Utilities|Array|Clear (Variables|Default|GetWood_Resource)))))

(fn CheckStone
  (bind _stone_resource (Variables|Default|GetStone_Resource))
  (bind _outactors (Actor|GetAllActorsOfClass "/Game/Blueprints/ResourceSpawner/BP_STONE1.BP_STONE1_C"))
  (for _array_element _outactors
    (if (<= (Transformation|GetDistanceTo _array_element) 7e+02)
      (Utilities|Array|Add (Variables|Default|GetStone_Resource) _array_element)))
  (for (_ _array_index) _stone_resource
    (if (<= (Transformation|GetDistanceTo (Utilities|Array|Get(acopy) _stone_resource _array_index)) 7e+02)
      (Default|RemoveStone (Utilities|Array|Get(acopy) _stone_resource _array_index))
      (bind _returnvalue (Actor|GetActorOfClass "/Game/MainGameModeBP/StrategyGameModeBase.StrategyGameModeBase_C"))
      (Default|AddStonetoMain _returnvalue)
      (Utilities|Array|Clear (Variables|Default|GetStone_Resource)))))