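; AngryAI is an AI-controlled enemy soldier that moves near a target, then shoots toward an Origin point.
; InitialPosition gathers actors of the Target class and sends the AI controller to one of the first four, randomly offset in X and Y.
; LookAtStructure waits, faces Origin and sets IsMoving.
; While that flag is set, Tick re-aims and spawns a Bullet roughly every second, throttled by a Delay.
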(event Custom|InitialPosition
  (bind _returnvalue (Math|Random|RandomFloatinRange -5e+02 5e+02))
  (bind _outactors (Actor|GetAllActorsOfClass "/Game/Blueprints/Old/Target.Target_C"))
  (bind _output_get (Variables|Default|SetTargetArray _outactors))
  (for _array_element _output_get
    (Utilities|Array|Add (Variables|Default|GetFinalTarget) _array_element))
  (AI|Navigation|MovetoLocation (AI|GetAIController self) (+ (Transformation|GetActorLocation (Utilities|Array|Get(acopy) (Variables|Default|GetFinalTarget) (Math|Random|RandomIntegerinRange 0 3))) (Math|Vector|MakeVector _returnvalue _returnvalue 0.0)) 5.0 false true false true 0))

(event Custom|LookAtStructure
  (Utilities|FlowControl|Delay 3.0)
  (Transformation|SetActorRotation (Math|Rotator|FindLookatRotation (Transformation|GetActorLocation self) (Variables|Default|GetOrigin)))
  (Variables|Default|SetisMoving true))

(event EventTick
  (params (DeltaSeconds :type Float%20%28single-precision%29))
  (Utilities|FlowControl|Delay 1.0)
  (if (Variables|Default|GetisMoving)
    (Transformation|SetActorRotation (Math|Rotator|FindLookatRotation (Transformation|GetActorLocation self) (Variables|Default|GetOrigin)))
    (Game|SpawnActorfromClass "/Game/Blueprints/Tank/Bullet.Bullet_C" (Transformation|GetActorTransform) "Undefined" 0 0)))

(fn ConstructionScript)