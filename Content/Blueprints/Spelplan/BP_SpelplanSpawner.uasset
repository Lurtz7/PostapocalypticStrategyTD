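; Game board spawner that builds a grid of tiles shortly after BeginPlay.
; InitieraElement spawns one tile at the origin, with its class picked at random from the child actors of a BP_Platta in the level.
; ByggVärld stores evenly spaced grid positions, then spawns PlattaA1 at each downward debug trace's end point, regardless of hits.
; An unconnected random switch over PlattaA tile variants remains in InitieraElement.
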(event EventBeginPlay
  (Utilities|FlowControl|Delay 0.2)
  (CallFunction|InitieraElement)
  (CallFunction|ByggVärld))

(fn ConstructionScript)

(fn InitieraElement
  (bind _returnvalue (Actor|GetActorOfClass "/Game/Blueprints/Spelplan/BP_Platta.BP_Platta_C"))
  (Game|SpawnActorfromClass (Utilities|GetClass (Utilities|Array|Get(acopy) (Actor|GetAllChildActors _returnvalue true) (Math|Random|RandomIntegerinRange 0 (Utilities|Array|Length (Actor|GetAllChildActors _returnvalue true))))) (Math|Transform|MakeTransform "0, 0, 0") "Undefined" 0 0))

(fn ByggVärld
  (bind _positions (Variables|Default|GetPositions))
  (for _index (range 0 5)
    (Variables|Default|SetY (+ (Variables|Default|GetY) 300))
    (for _index_2 (range 0 5)
      (Variables|Default|SetX (+ (Variables|Default|GetX) 300))
      (bind _output_get (Variables|Default|SetPosition (Math|Vector|MakeVector (Math|Conversions|ToFloat(Integer) (Variables|Default|GetX)) (Math|Conversions|ToFloat(Integer) (Variables|Default|GetY)) 0.0)))
      (Utilities|Array|Add _positions _output_get))
    (Variables|Default|SetX 0))
  (for _array_element _positions
    (bind _outhit (Collision|LineTraceByChannel (Math|Vector|MakeVector (.X (Math|Vector|BreakVector _array_element)) (.Y (Math|Vector|BreakVector _array_element)) 5e+02) (Math|Vector|MakeVector (.X (Math|Vector|BreakVector _array_element)) (.Y (Math|Vector|BreakVector _array_element)) 0.0) "TraceTypeQuery1" false 0 "Persistent"))
    (Game|SpawnActorfromClass "/Game/Blueprints/Spelplan/PlattaA1.PlattaA1_C" (Math|Transform|MakeTransform (.TraceEnd (Collision|BreakHitResult _outhit))) "Undefined" 0 0)))