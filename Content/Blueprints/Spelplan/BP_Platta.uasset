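; BP_Platta is a game-board (Spelplan) plate Blueprint that spawns its items as child actors at runtime.
; On BeginPlay it adds eight Child Actor Components in a hardcoded, unrolled sequence with automatic attachment.
; Each new component is written into ArrayOfItems with an array Set rather than an Add.
; The Construction Script is empty, so these components are created only once play begins.
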(event EventBeginPlay
  (bind _arrayofitems (Variables|Default|GetArrayOfItems))
  (bind _returnvalue (AddComponent|AddChildActorComponent false))
  (Utilities|Array|SetArrayElem _arrayofitems 0 _returnvalue)
  (bind _returnvalue_2 (AddComponent|AddChildActorComponent false))
  (Utilities|Array|SetArrayElem _arrayofitems 0 _returnvalue_2)
  (bind _returnvalue_3 (AddComponent|AddChildActorComponent false))
  (Utilities|Array|SetArrayElem _arrayofitems 0 _returnvalue_3)
  (bind _returnvalue_4 (AddComponent|AddChildActorComponent false))
  (Utilities|Array|SetArrayElem _arrayofitems 0 _returnvalue_4)
  (bind _returnvalue_5 (AddComponent|AddChildActorComponent false))
  (Utilities|Array|SetArrayElem _arrayofitems 0 _returnvalue_5)
  (bind _returnvalue_6 (AddComponent|AddChildActorComponent false))
  (Utilities|Array|SetArrayElem _arrayofitems 0 _returnvalue_6)
  (bind _returnvalue_7 (AddComponent|AddChildActorComponent false))
  (Utilities|Array|SetArrayElem _arrayofitems 0 _returnvalue_7)
  (bind _returnvalue_8 (AddComponent|AddChildActorComponent false))
  (Utilities|Array|SetArrayElem _arrayofitems 0 _returnvalue_8))

(fn ConstructionScript)