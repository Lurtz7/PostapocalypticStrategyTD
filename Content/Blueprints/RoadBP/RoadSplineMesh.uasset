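; Road spline actor that lays out a straight line of spline points in its Construction Script.
; A loop appends points to RoadSpline in local space, stepping the SplinePositions variable along X each time.
; A disconnected section, which never runs, would tile spline mesh components along the spline at Distance intervals, with tangents scaled from the spline direction.
; The event graph has no active logic.
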(event EventBeginPlay)

(event Collision|EventActorBeginOverlap
  (params (OtherActor :type Actor%20Object%20Reference)))

(event EventTick
  (params (DeltaSeconds :type Float%20%28single-precision%29)))

(fn ConstructionScript
  (for _index (range 0 10)
    (Spline|AddSplinePoint (Variables|Default|GetRoadSpline) (Math|Vector|MakeVector (.X (Math|Vector|BreakVector (Variables|Default|GetSplinePositions))) (.Y (Math|Vector|BreakVector (Variables|Default|GetSplinePositions))) (.Z (Math|Vector|BreakVector (Variables|Default|GetSplinePositions)))) "Local" true)
    (Variables|Default|SetSplinePositions (Math|Vector|MakeVector (+ (.X (Math|Vector|BreakVector (Variables|Default|GetSplinePositions))) 1e+02) (.Y (Math|Vector|BreakVector (Variables|Default|GetSplinePositions))) (.Z (Math|Vector|BreakVector (Variables|Default|GetSplinePositions)))))))